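; BP_DamageBox is a hazard volume that hurts the third-person player character while it stands inside the box.
; On begin overlap it stores the BP_ThirdPersonCharacter, applies damage at once and starts a looping timer that reapplies the same damage at a fixed interval.
; On end overlap with that character type it clears and invalidates the stored timer handle, stopping the damage.
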(event OnComponentBeginOverlap(Box)
  (params (OverlappedComponent :type Primitive%20Component%20Object%20Reference) (OtherActor :type Actor%20Object%20Reference) (OtherComp :type Primitive%20Component%20Object%20Reference) (OtherBodyIndex :type Integer) (bFromSweep :type Boolean) (SweepResult :type Hit%20Result%20Structure%20%28by%20ref%29))
  (bind _asbp_third_person_character (Utilities|Casting|CastToBP_ThirdPersonCharacter OtherActor))
  (bind _output_get (Variables|Default|SetThirdPesonPlayerCharacter _asbp_third_person_character))
  (Game|Damage|ApplyDamage _output_get 1e+01 0 0)
  (bind _returnvalue (Utilities|Time|SetTimerbyEvent (delegate Custom|OnPlayerOnDamageBox) 1.5 true))
  (Variables|Default|SetHealthTimerEvent _returnvalue))

(event OnComponentEndOverlap(Box)
  (params (OverlappedComponent :type Primitive%20Component%20Object%20Reference) (OtherActor :type Actor%20Object%20Reference) (OtherComp :type Primitive%20Component%20Object%20Reference) (OtherBodyIndex :type Integer))
  (Utilities|Casting|CastToBP_ThirdPersonCharacter OtherActor)
  (Utilities|Time|ClearandInvalidateTimerbyHandle (Variables|Default|GetHealthTimerEvent)))

(event Custom|OnPlayerOnDamageBox
  (Game|Damage|ApplyDamage (Variables|Default|GetThirdPesonPlayerCharacter) 1e+01 0 0))

(fn ConstructionScript)