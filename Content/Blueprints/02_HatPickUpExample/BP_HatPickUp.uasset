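; Hat pickup actor that the third-person character can collect by pressing E while inside its sphere trigger.
; Sphere overlap stores the BP_ThirdPersonCharacter and enables input for player 0; leaving clears the reference and calls DisableInput.
; Pressing E with a valid character passes SM_Hat to its OnHatPickedUp, then destroys the pickup.
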(event OnComponentBeginOverlap(Sphere)
  (params (OverlappedComponent :type Primitive%20Component%20Object%20Reference) (OtherActor :type Actor%20Object%20Reference) (OtherComp :type Primitive%20Component%20Object%20Reference) (OtherBodyIndex :type Integer) (bFromSweep :type Boolean) (SweepResult :type Hit%20Result%20Structure%20%28by%20ref%29))
  (bind _asbp_third_person_character (Utilities|Casting|CastToBP_ThirdPersonCharacter OtherActor))
  (Variables|Default|SetThirdPersonCharacter _asbp_third_person_character)
  (Input|EnableInput (Game|GetPlayerController 0)))

(event OnComponentEndOverlap(Sphere)
  (params (OverlappedComponent :type Primitive%20Component%20Object%20Reference) (OtherActor :type Actor%20Object%20Reference) (OtherComp :type Primitive%20Component%20Object%20Reference) (OtherBodyIndex :type Integer))
  (if (== OtherActor (Variables|Default|GetThirdPersonCharacter))
    (Variables|Default|SetThirdPersonCharacter 0)
    (Input|DisableInput (Game|GetPlayerController 0) 0)))

(event Input|KeyboardEvents|E
  (params (Key :type Key%20Structure :default "None"))
  (:Pressed
    (bind _thirdpersoncharacter (Variables|Default|GetThirdPersonCharacter)
      (:then
        (Default|OnHatPickedUp _thirdpersoncharacter "/Game/Beginner_Blueprints/Course_Assets/SM_Hat.SM_Hat")
        (Actor|DestroyActor))
      (:else))))

(fn ConstructionScript)