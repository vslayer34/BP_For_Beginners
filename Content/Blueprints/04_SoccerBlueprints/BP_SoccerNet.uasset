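; BP_SoccerNet is a soccer goal that detects a BP_SoccerBall entering its box trigger and respawns the ball.
; On overlap it plays a hit emitter above the net and disables the trigger, then after short delays hides and destroys the ball.
; It spawns a fresh ball at a location cached on BeginPlay from a referenced location actor, then re-enables the trigger.
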(event OnComponentBeginOverlap(Box)
  (params (OverlappedComponent :type Primitive%20Component%20Object%20Reference) (OtherActor :type Actor%20Object%20Reference) (OtherComp :type Primitive%20Component%20Object%20Reference) (OtherBodyIndex :type Integer) (bFromSweep :type Boolean) (SweepResult :type Hit%20Result%20Structure%20%28by%20ref%29))
  (bind _returnvalue (Transformation|GetActorLocation))
  (bind _asbp_soccer_ball (Utilities|Casting|CastToBP_SoccerBall OtherActor))
  (Variables|Default|SetSoccerBall _asbp_soccer_ball)
  (Effects|SpawnEmitteratLocation "/Game/FXVarietyPack/Particles/P_ky_hit1.P_ky_hit1" (Math|Vector|MakeVector (.x _returnvalue) (.y _returnvalue) (+ (.z _returnvalue) 3e+02)))
  (Collision|SetCollisionEnabled (Variables|Default|GetBox) "NoCollision")
  (Utilities|FlowControl|Delay 1.5)
  (Rendering|SetActorHiddenInGame (Variables|Default|GetSoccerBall) true)
  (Utilities|FlowControl|Delay 1.0)
  (Actor|DestroyActor (Variables|Default|GetSoccerBall))
  (Game|SpawnActorfromClass "/Game/Blueprints/04_SoccerBlueprints/BP_SoccerBall.BP_SoccerBall_C" (Math|Transform|MakeTransform (Variables|Default|GetBallSpawnLocation) "0, 0, 0" "1.000000,1.000000,1.000000") "Undefined" "MultiplyWithRoot" 0 0)
  (Collision|SetCollisionEnabled (Variables|Default|GetBox) "QueryOnly"))

(event EventBeginPlay
  (bind _soccerballlocation (Variables|Default|GetSoccerBallLocation)
    (:then
      (Variables|Default|SetBallSpawnLocation (Transformation|GetActorLocation _soccerballlocation)))
    (:else)))

(fn ConstructionScript)